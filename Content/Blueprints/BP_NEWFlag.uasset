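; BP_NEWFlag is a capture-point flag that either the water or fire team can claim.
; Each WaterFlag or FireFlag call spawns that team's ball emitter if neither exists, then moves it by a shared Height using speeds set through SetSpeed.
; Height 3000 spawns a team circle effect and sets Flagteam, while dropping to zero clears both.
; Overlap-based controller tracking is present but disconnected.
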(event `generate water flag`
  ;[1 1 1] 生成旗帜
  (`/Engine/EditorBlueprintResources/StandardMacros.IsValid` (`self.fire emitter`)
    (:`Is Not Valid`
      (`/Engine/EditorBlueprintResources/StandardMacros.IsValid` (`self.water emitter`)
        (:`Is Not Valid`
          (bind _returnvalue (`GameplayStatics.SpawnEmitterAtLocation` "/Game/FXVarietyPack/Particles/P_ky_waterBall.P_ky_waterBall" (`SceneComponent.K2_GetComponentLocation` (`self.flag`)) (struct) (1.0 1.0 1.0) false))
          (set `self.water emitter` _returnvalue))))))

(event `generate fire flag`
  ;[1 1 1] 生成旗帜
  (`/Engine/EditorBlueprintResources/StandardMacros.IsValid` (`self.fire emitter`)
    (:`Is Not Valid`
      (`/Engine/EditorBlueprintResources/StandardMacros.IsValid` (`self.water emitter`)
        (:`Is Not Valid`
          (bind _returnvalue (`GameplayStatics.SpawnEmitterAtLocation` "/Game/FXVarietyPack/Particles/P_ky_fireBall.P_ky_fireBall" (`SceneComponent.K2_GetComponentLocation` (`self.flag`)) (struct) (1.0 1.0 1.0) false))
          (set `self.fire emitter` _returnvalue))))))

(event `water team flag`
  (bind _water_circle (`self.water circle`))
  (bind _flag (`self.flag`))
  (bind _water_emitter (`self.water emitter`))
  ;[1 1 1] 旗子的上升与下降
  ;;[1 1 1] water
  (`self.generate water flag`)
  (`/Engine/EditorBlueprintResources/StandardMacros.IsValid` (`self.water emitter`)
    (:`Is Valid`
      (set `self.height ` (+ (`self.height `) (`self.water speed`)))
      (`SceneComponent.K2_SetWorldLocation` (`self.water emitter`) (+ (`SceneComponent.K2_GetComponentLocation` _flag) (* (`KismetMathLibrary.GetUpVector` (`SceneComponent.K2_GetComponentRotation` _flag)) (/ (`self.height `) 4))) false false)
      (if (<= (`self.height `) 0)
        ;;[1 1 1] water占领被结束
        (set `self.water complete` false)
        (`|ExecutionSequence`
          (:`then_0`
            (`/Engine/EditorBlueprintResources/StandardMacros.IsValid` _water_emitter
              (:`Is Valid`
                (`ActorComponent.K2_DestroyComponent` _water_emitter)
                (set `self.water complete` false)
                (set `self.flagteam` 0))))
          (:`then_1`
            (`/Engine/EditorBlueprintResources/StandardMacros.IsValid` _water_circle
              (:`Is Valid`
                (`ActorComponent.K2_DestroyComponent` _water_circle)))))
        (else
          ;;[1 1 1] water 完成占领
          (if (>= (`self.height `) 3000)
            (if (not (`self.water complete`))
              (bind _returnvalue (`GameplayStatics.SpawnEmitterAtLocation` "/Game/FXVarietyPack/Particles/flag_water.flag_water" (`SceneComponent.K2_GetComponentLocation` (`self.flag`)) (struct) (2.0 2.0 2.0) false))
              (set `self.water circle` _returnvalue)
              (set `self.water complete` true)
              (bind _output_get (set `self.flagteam` 1))
              (`KismetSystemLibrary.PrintString` (`KismetStringLibrary.Conv_IntToString` _output_get)))))))))

(event `fire team flag`
  (bind _fire_circle (`self.fire circle`))
  (bind _flag (`self.flag`))
  (bind _fire_emitter (`self.fire emitter`))
  ;[1 1 1] 旗子的上升与下降
  ;;[1 1 1] Fire
  (`self.generate fire flag`)
  (`/Engine/EditorBlueprintResources/StandardMacros.IsValid` (`self.fire emitter`)
    (:`Is Valid`
      (set `self.height ` (+ (`self.height `) (`self.firespeed`)))
      (`SceneComponent.K2_SetWorldLocation` (`self.fire emitter`) (+ (`SceneComponent.K2_GetComponentLocation` _flag) (* (`KismetMathLibrary.GetUpVector` (`SceneComponent.K2_GetComponentRotation` _flag)) (/ (`self.height `) 4))) false false)
      (if (<= (`self.height `) 0)
        (set `self.fire complete` false)
        ;;[1 1 1] fire占领被结束
        (`|ExecutionSequence`
          (:`then_0`
            (`/Engine/EditorBlueprintResources/StandardMacros.IsValid` _fire_circle
              (:`Is Valid`
                (`ActorComponent.K2_DestroyComponent` _fire_circle)
                (set `self.fire complete` false)
                (set `self.flagteam` 0))))
          (:`then_1`
            (`/Engine/EditorBlueprintResources/StandardMacros.IsValid` _fire_emitter
              (:`Is Valid`
                (`ActorComponent.K2_DestroyComponent` _fire_emitter)))))
        (else
          ;;[1 1 1] fire 完成占领
          (if (>= (`self.height `) 3000)
            (if (not (`self.fire complete`))
              (bind _returnvalue (`GameplayStatics.SpawnEmitterAtLocation` "/Game/FXVarietyPack/Particles/flag_fire.flag_fire" (`SceneComponent.K2_GetComponentLocation` (`self.flag`)) (struct) (2.0 2.0 2.0) false))
              (set `self.fire circle` _returnvalue)
              (set `self.fire complete` true)
              (set `self.flagteam` 2))))))))

(event `self.FireFlag`
  (`self.fire team flag`))

(event `self.WaterFlag`
  (`self.water team flag`))

(event `self.SetSpeed`
  (params (speed :type Integer))
  (`|ExecutionSequence`
    (:`then_0`
      (set `self.firespeed` speed))
    (:`then_1`
      (set `self.water speed` speed))))

(event `self.flag.OnComponentBeginOverlap`
  (params (OverlappedComponent :type "PrimitiveComponent Object Reference") (OtherActor :type "Actor Object Reference") (OtherComp :type "PrimitiveComponent Object Reference") (OtherBodyIndex :type Integer) (bFromSweep :type Boolean) (SweepResult :type "HitResult Structure (by ref)"))
  ;[1 1 1] 查询人数
)

(event `self.Box.OnComponentEndOverlap`
  (params (OverlappedComponent :type "PrimitiveComponent Object Reference") (OtherActor :type "Actor Object Reference") (OtherComp :type "PrimitiveComponent Object Reference") (OtherBodyIndex :type Integer))
  ;[1 1 1] 查询人数
)

(event `self.ReceiveTick`
  (params (DeltaSeconds :type "Float (single-precision)"))
  ;[1 1 1] 查询人数
)

(fn `UserConstructionScript`)