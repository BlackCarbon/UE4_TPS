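; BP_WiterProjectile is a water projectile that deals damage to what it hits in a third-person shooter.
; On Hit it forwards to a water-hit event, commented as networked, which applies stream-randomized point damage, triggers a water-ball impact emitter and destroys the projectile.
; TPSCharacter hits also pass the instigator controller.
; A constant-true branch damages every other actor, leaving the fallback actor-spawn path unreachable.
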(event `self.ReceiveHit`
  (params (MyComp :type "PrimitiveComponent Object Reference") (Other :type "Actor Object Reference") (OtherComp :type "PrimitiveComponent Object Reference") (bSelfMoved :type Boolean) (HitLocation :type "Vector Structure") (HitNormal :type "Vector Structure") (NormalImpulse :type "Vector Structure") (Hit :type "HitResult Structure (by ref)"))
  ;[1 1 1] 联网
  (`self.TPS_waterHit` Hit))

(event `TPS_waterHit`
  (params (Hit :type "HitResult Structure (by ref)"))
  (bind (_bblockinghit _binitialoverlap _time _distance _location _impactpoint _normal _impactnormal _physmat _hitactor) (`GameplayStatics.BreakHitResult` Hit))
  (if (`KismetMathLibrary.ClassIsChildOf` (`GameplayStatics.GetObjectClass` _hitactor) "/Script/TPS.TPSCharacter")
    ;[1 1 1] 如果撞击的对象是character
    (`GameplayStatics.ApplyPointDamage` _hitactor (`KismetMathLibrary.RandomFloatInRangeFromStream` 15.0 10.0 (`self.Random Dange String`)) _location Hit (`self.GetInstigatorController`) self)
    (`self.TPS fire_effect` _location)
    (`self.K2_DestroyActor` self)
    (elif true
      ;[1 1 1] 撞击到能破坏的Actor
      (`GameplayStatics.ApplyPointDamage` _hitactor (`KismetMathLibrary.RandomFloatInRangeFromStream` 15.0 10.0 (`self.Random Dange String`)) _location Hit null self)
      (`self.TPS fire_effect` _location)
      (`self.K2_DestroyActor`)
      (else
        (bind _returnvalue (`|SpawnActorFromClass` "/Script/Engine.Actor" (`self.GetTransform`) "Undefined" "OverrideRootScale" null null))
        (`self.K2_AddActorWorldOffset` _returnvalue _location false false)
        (`self.K2_DestroyActor`)))))

(event `TPS fire_effect`
  (params (Location :type "Vector Structure"))
  (`GameplayStatics.SpawnEmitterAtLocation` "/Game/FXVarietyPack/Particles/P_ky_waterBallHit.P_ky_waterBallHit" Location))

(fn `UserConstructionScript`)